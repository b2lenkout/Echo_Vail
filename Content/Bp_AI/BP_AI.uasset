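; BP_AI is an enemy character that chases the player and melee-attacks with a bat.
; ChasePlayer moves to the player, triggers Attack on arrival, then repeats after a short delay.
; Attack plays the slash montage, sphere-traces at the hand socket on its notify to damage the player, and calls OnAttackEnd when finished or interrupted.
; AttackBat spawns and attaches the bat; BeginPlay is empty, so nothing here starts the behavior.
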(event `self.ReceiveBeginPlay`)

(event `ChasePlayer`
  (`|AIMoveTo` self (0.0 0.0 0.0) (`GameplayStatics.GetPlayerCharacter` 0) 150.0
    (:`OnSuccess`
      (`self.Attack`)
      (`KismetSystemLibrary.Delay` 1.0)
      (`self.ChasePlayer`))))

(event `Attack`
  (bind _returnvalue (`SceneComponent.GetSocketLocation` (`self.Mesh`) "ik_hand_rBatSocket"))
  (`|PlayMontage` (`self.Mesh`) "/Game/Bp_AI/MontageBatSlash.MontageBatSlash"
    (:`OnCompleted`
      (`self.OnAttackEnd` :!label _label))
    (:`OnInterrupted`
      (goto _label))
    (:`OnNotifyBegin`
      (bind _outhit (`KismetSystemLibrary.SphereTraceSingleForObjects` :`Start` _returnvalue :`End` _returnvalue :`Radius` 50.0 :`ObjectTypes` (`|MakeArray` "ObjectTypeQuery3" :!type "EObjectTypeQuery Enum") :`DrawDebugType` "ForDuration"))
      (bind _asbp_third_person_character (cast `/Game/ThirdPerson/Blueprints/BP_ThirdPersonCharacter` (`.HitActor` (`GameplayStatics.BreakHitResult` _outhit))))
      (`GameplayStatics.ApplyDamage` _asbp_third_person_character 34.0))))

(event `AttackBat`
  (bind _returnvalue (`|SpawnActorFromClass` "/Game/Weapons/Bp_Bat.Bp_Bat_C" (`self.GetTransform`) "Undefined" "MultiplyWithRoot" null null))
  (`self.K2_AttachToComponent` _returnvalue (`self.Mesh`) "ik_hand_rBatSocket" "SnapToTarget" "SnapToTarget" "SnapToTarget" true)
  (set `self.isAttackingBat` true))

(fn `UserConstructionScript`)